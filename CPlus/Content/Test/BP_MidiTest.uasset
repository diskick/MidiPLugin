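; BP_MidiTest is a test Blueprint that plays the Yuanshen MIDI through two synth tone generator components.
; On BeginPlay it binds to the MIDI's note-on event, then starts playback after a short delay.
; Each note number is converted to an equal-tempered frequency and printed.
; Track 1 notes sound on the first generator for the event's Time, while track 2 notes use the second for a fixed length.
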(event Custom|OnNoteOnEvent_事件
  (params (event :type Midi%20Event%20Structure))
  (bind (_time _note _velocity _bplayed _intrack) (Utilities|Struct|BreakMidiEvent event))
  (bind _synthcomponenttonegenerator1 (Variables|Default|GetSynthComponentToneGenerator1))
  (bind _synthcomponenttonegenerator (Variables|Default|GetSynthComponentToneGenerator))
  (bind _returnvalue (- _note 69))
  (bind _returnvalue_2 (Math|Conversions|ToFloat(Integer) _returnvalue))
  (bind _returnvalue_3 (/ _returnvalue_2 12.0))
  (bind _returnvalue_4 (Math|Float|Power 2.0 _returnvalue_3))
  (bind _returnvalue_5 (* _returnvalue_4 4.4e+02))
  (Development|PrintString (Utilities|String|ToString(Float) _returnvalue_5))
  (switch int _intrack
    (:1
      (Class|SynthComponentToneGenerator|SetFrequency _synthcomponenttonegenerator _returnvalue_5)
      (CameraShake|Start _synthcomponenttonegenerator)
      (Utilities|FlowControl|Delay _time)
      (Audio|Components|Audio|Stop _synthcomponenttonegenerator))
    (:2
      (Class|SynthComponentToneGenerator|SetFrequency _synthcomponenttonegenerator1 _returnvalue_5)
      (CameraShake|Start _synthcomponenttonegenerator1)
      (Utilities|FlowControl|Delay 0.2)
      (Audio|Components|Audio|Stop _synthcomponenttonegenerator1))))

(event EventBeginPlay
  (bind _output_get (Variables|Default|SetMidi "/Game/Test/yuanshen.yuanshen"))
  (EventDispatchers|AssignOnNoteonEvent _output_get (delegate Custom|OnNoteOnEvent_事件))
  (Utilities|FlowControl|Delay 2.0)
  (Class|MidiAsset|Playnotes _output_get (stale EventTick DeltaSeconds)))

(event EventTick
  (params (DeltaSeconds :type Float%20%28single-precision%29)))

(fn ConstructionScript)